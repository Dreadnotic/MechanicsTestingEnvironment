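; Pushable cube Blueprint that the mouse character (MouseBP) can shove.
; The X_Push and Y_Push overlap volumes both set a shared Overlapping flag when that character's capsule enters or leaves.
; While overlapping, Tick turns the cube's physics simulation on or off to follow MouseBP.PushingCube.
; Physics constraint calls for locking or freeing the X and Y axes are present but disconnected, so push direction is not restricted here.
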(event OnComponentBeginOverlap(Y_Push)
  (params (OverlappedComponent :type Primitive%20Component%20Object%20Reference) (OtherActor :type Actor%20Object%20Reference) (OtherComp :type Primitive%20Component%20Object%20Reference) (OtherBodyIndex :type Integer) (bFromSweep :type Boolean) (SweepResult :type Hit%20Result%20Structure%20%28by%20ref%29))
  (if (== OtherComp (Variables|/Script/Engine.Character|GetCapsuleComponent (Variables|Default|GetMouseBP)))
    (Variables|Default|SetOverlapping true)))

(event OnComponentEndOverlap(Y_Push)
  (params (OverlappedComponent :type Primitive%20Component%20Object%20Reference) (OtherActor :type Actor%20Object%20Reference) (OtherComp :type Primitive%20Component%20Object%20Reference) (OtherBodyIndex :type Integer))
  (if (== OtherComp (Variables|/Script/Engine.Character|GetCapsuleComponent (Variables|Default|GetMouseBP)))
    (Variables|Default|SetOverlapping false)))

(event OnComponentBeginOverlap(X_Push)
  (params (OverlappedComponent :type Primitive%20Component%20Object%20Reference) (OtherActor :type Actor%20Object%20Reference) (OtherComp :type Primitive%20Component%20Object%20Reference) (OtherBodyIndex :type Integer) (bFromSweep :type Boolean) (SweepResult :type Hit%20Result%20Structure%20%28by%20ref%29))
  (if (== OtherComp (Variables|/Script/Engine.Character|GetCapsuleComponent (Variables|Default|GetMouseBP)))
    (Variables|Default|SetOverlapping true)))

(event OnComponentEndOverlap(X_Push)
  (params (OverlappedComponent :type Primitive%20Component%20Object%20Reference) (OtherActor :type Actor%20Object%20Reference) (OtherComp :type Primitive%20Component%20Object%20Reference) (OtherBodyIndex :type Integer))
  (if (== OtherComp (Variables|/Script/Engine.Character|GetCapsuleComponent (Variables|Default|GetMouseBP)))
    (Variables|Default|SetOverlapping false)))

(event EventTick
  (params (DeltaSeconds :type Float%20%28single-precision%29))
  (bind _cube (Variables|Default|GetCube))
  (if (Variables|Default|GetOverlapping)
    (if (Variables|/Game/MouseCharacter/MouseCharacter.MouseCharacter_C|GetPushingCube (Variables|Default|GetMouseBP))
      (Physics|SetSimulatePhysics _cube true)
      (else
        (Physics|SetSimulatePhysics _cube false)))))

(fn ConstructionScript)