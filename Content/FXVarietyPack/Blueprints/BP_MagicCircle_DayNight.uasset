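; Magic circle teleport pad that belongs to either day or night, set by its DayTP or NightTP actor tag.
; At BeginPlay it gathers circles with the opposite tag and binds to MouseCharacter's day/night switch, which activates or deactivates its effect.
; During its own phase, the character's capsule entering or leaving the sphere sends teleport toggle messages to the character and those opposite circles, whose effects can thereby toggle.
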(event OnComponentActivated(fx)
  (params (Component :type Actor%20Component%20Object%20Reference) (bReset :type Boolean))
  (if (Math|Boolean|Equal(Boolean) (Variables|Default|GetDayOrNight) (Variables|Default|GetIsDay?))
    (Effects|Components|ParticleSystem|SetVectorParameter (Variables|Default|Getfx) "color" (Math|Conversions|ToVector(LinearColor) (Variables|Default|GetDefaultColor)))))

(event OnComponentBeginOverlap(Sphere)
  (params (OverlappedComponent :type Primitive%20Component%20Object%20Reference) (OtherActor :type Actor%20Object%20Reference) (OtherComp :type Primitive%20Component%20Object%20Reference) (OtherBodyIndex :type Integer) (bFromSweep :type Boolean) (SweepResult :type Hit%20Result%20Structure%20%28by%20ref%29))
  (bind _dayornight (Variables|Default|GetDayOrNight))
  (bind _isday_ (Variables|Default|GetIsDay?))
  (bind _returnvalue (Math|Boolean|Equal(Boolean) _isday_ _dayornight))
  (if _returnvalue
    (Development|PrintString (Utilities|String|Append "BoolA: " (Utilities|String|ToString(Boolean) _dayornight) " BoolB: " (Utilities|String|ToString(Boolean) _isday_) " Outcome:" (Utilities|String|ToString(Boolean) _returnvalue)) true true "(R=0.000000,G=0.660000,B=1.000000,A=1.000000)" (Utilities|Time|GetWorldDeltaSeconds))
    (bind _asmouse_character (Utilities|Casting|CastToMouseCharacter OtherActor))
    (if (== OtherComp (Variables|/Script/Engine.Character|GetCapsuleComponent _asmouse_character))
      (Class|SwitchInterface|2WayTeleToggle(Message) _asmouse_character)
      (for _array_element (Variables|Default|GetTargetArray)
        (Class|SwitchInterface|TeleportToggle(Message) _array_element)))))

(event OnComponentEndOverlap(Sphere)
  (params (OverlappedComponent :type Primitive%20Component%20Object%20Reference) (OtherActor :type Actor%20Object%20Reference) (OtherComp :type Primitive%20Component%20Object%20Reference) (OtherBodyIndex :type Integer))
  (if (Math|Boolean|Equal(Boolean) (Variables|Default|GetDayOrNight) (Variables|Default|GetIsDay?))
    (bind _asmouse_character (Utilities|Casting|CastToMouseCharacter OtherActor))
    (if (== OtherComp (Variables|/Script/Engine.Character|GetCapsuleComponent _asmouse_character))
      (Class|SwitchInterface|2WayTeleToggle(Message) _asmouse_character)
      (for _array_element (Variables|Default|GetTargetArray)
        (Class|SwitchInterface|TeleportToggle(Message) _array_element)))))

(event Custom|DayNightToggle
  (bind _fx (Variables|Default|Getfx))
  (Variables|Default|SetIsDay? (not (Variables|Default|GetIsDay?)))
  (if (Variables|Default|GetDayOrNight)
    (if (Variables|Default|GetIsDay?)
      (Components|Activation|Activate _fx false :!label _label)
      (else
        (Components|Activation|Deactivate _fx :!label _label_2)))
    (elif (Variables|Default|GetIsDay?)
      (goto _label_2)
      (else
        (goto _label)))))

(event EventBeginPlay
  (|CallParentFunction)
  (bind _asmouse_character (Utilities|Casting|CastToMouseCharacter (Game|GetPlayerCharacter 0)))
  (EventDispatchers|BindEventtoDayNightSwitch _asmouse_character (delegate Custom|DayNightToggle))
  (bind _output_get (Variables|Default|SetDayOrNight (Actor|ActorHasTag "DayTP")))
  (if _output_get
    (bind _outactors (Actor|GetAllActorsOfClasswithTag "BP_MagicCircle_DayNight_C" "NightTP"))
    (Development|PrintString "GotNightTimeTags")
    (Variables|Default|SetTargetArray _outactors)
    (else
      (bind _outactors_2 (Actor|GetAllActorsOfClasswithTag "BP_MagicCircle_DayNight_C" "DayTP"))
      (Development|PrintString "GotDayTimeTags")
      (Variables|Default|SetTargetArray _outactors_2)
      (Components|Activation|Deactivate (Variables|Default|Getfx)))))

(event Collision|EventActorBeginOverlap
  (params (OtherActor :type Actor%20Object%20Reference))
  (|CallParentFunction OtherActor) ; This node is disabled and will not be called.\nDrag off pins to build functionality.
)

(event EventTick
  (params (DeltaSeconds :type Float%20%28single-precision%29))
  (|CallParentFunction DeltaSeconds))

(event EventTeleportToggle
  (Components|Activation|ToggleActive (Variables|Default|Getfx)))

(event EventTeleportColor
  (Development|PrintString "Color Set!")
  (Effects|Components|ParticleSystem|SetVectorParameter (Variables|Default|Getfx) "color" (Math|Conversions|ToVector(LinearColor) (select (Variables|Default|GetIsColorSet?) (Variables|Default|GetDefaultColor) (Utilities|Struct|MakeLinearColor 0.0 255.0 0.0 0.3))))
  (if (Variables|Default|GetIsColorSet?)
    (Variables|Default|SetIsColorSet? false)
    (else
      (Variables|Default|SetIsColorSet? true))))

(fn ConstructionScript
  (bind _color (Variables|Default|Getcolor))
  (|CallParentFunction)
  (Effects|Components|ParticleSystem|SetVectorParameter (Variables|Default|Getfx) "color" (Math|Conversions|ToVector(LinearColor) _color))
  (Variables|Default|SetDefaultColor _color))